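; BP_Goal is a ring goal that reports to its goal manager when a character passes through it from an accepted direction.
; Init stores the manager and index, and the construction script rotates the ring and collider to an initial yaw.
; On overlap, it requires a CharacterMovementComponent and an impact normal within an angular tolerance of the collider's reversed forward vector, then calls GoalPassed with its index.
; The check also prints the measured angle.
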(event OnComponentBeginOverlap(Collider)
  (params (OverlappedComponent :type Primitive%20Component%20Object%20Reference) (OtherActor :type Actor%20Object%20Reference) (OtherComp :type Primitive%20Component%20Object%20Reference) (OtherBodyIndex :type Integer) (bFromSweep :type Boolean) (SweepResult :type Hit%20Result%20Structure%20%28by%20ref%29))
  (bind _isvalid (CallFunction|CheckValidCollision SweepResult OtherActor))
  (if _isvalid
    (Default|GoalPassed (Variables|Default|GetmyGoalManager) (Variables|Default|Getindex))))

(event EventBeginPlay)

(event Collision|EventActorBeginOverlap
  (params (OtherActor :type Actor%20Object%20Reference)))

(event EventTick
  (params (DeltaSeconds :type Float%20%28single-precision%29)))

(fn ConstructionScript
  (bind _initial_rot (Variables|Default|GetInitial%20Rot))
  (Transformation|SetRelativeRotation (Variables|Default|GetNS_Ring) (Math|Rotator|MakeRotator 0.0 0.0 _initial_rot) false false)
  (Transformation|SetRelativeRotation (Variables|Default|GetCollider) (Math|Rotator|MakeRotator 9e+01 0.0 _initial_rot) false false))

(fn GetIndex
  (return (Variables|Default|Getindex)))

(fn GetGoalMNGR
  (return (Variables|Default|GetmyGoalManager)))

(fn Init
  (params (GoalMNGR :type BP%20Goal%20Manager%20Object%20Reference) (Index :type Integer))
  (Variables|Default|Setindex Index)
  (Variables|Default|SetmyGoalManager GoalMNGR))

(fn CheckValidCollision
  (params (Hit :type Hit%20Result%20Structure%20%28by%20ref%29) (other :type Actor%20Object%20Reference))
  (bind _impactnormal (Collision|BreakHitResult Hit))
  (bind _collider (Variables|Default|GetCollider))
  (bind _returnvalue (Math|Vector|GetForwardVector _collider))
  (bind _returnvalue_2 (* _returnvalue "-1.000000,-1.000000,-1.000000"))
  (bind _returnvalue_3 (Math|Vector|DotProduct _returnvalue_2 _impactnormal))
  (bind _returnvalue_4 (Class|KismetMathLibrary|DegAcos _returnvalue_3))
  (Development|PrintString (Utilities|String|ToString(Float) _returnvalue_4))
  (return (and (Utilities|IsValid (Actor|GetComponentbyClass other "/Script/Engine.CharacterMovementComponent")) (< _returnvalue_4 (Variables|Default|Gettolerance)))))