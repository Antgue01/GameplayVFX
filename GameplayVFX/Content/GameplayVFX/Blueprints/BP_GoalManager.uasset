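; BP_GoalManager runs an ordered goal course, timing the run and awarding a trophy at the end.
; Reset initializes each goal with its index, shows only the first NumActive goals, and records the start time.
; GoalPassed accepts only the current goal, hiding it and revealing the one NumActive ahead as a sliding window.
; FinalGoallPassed hides the manager and passes elapsed time to TrophyManager when the last goal is current.
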(event EventBeginPlay
  (CallFunction|Reset true))

(event Collision|EventActorBeginOverlap
  (params (OtherActor :type Actor%20Object%20Reference)))

(event EventTick
  (params (DeltaSeconds :type Float%20%28single-precision%29)))

(fn ConstructionScript)

(fn GoalPassed
  (params (goalIndex :type Integer))
  (bind _goals (Variables|Default|Getgoals))
  (bind _numactive (Variables|Default|GetnumActive))
  (bind _returnvalue (+ goalIndex _numactive))
  (if (== goalIndex (Variables|Default|GetcurrentGoal))
    (Rendering|SetActorHiddenInGame (Utilities|Array|Get(acopy) _goals goalIndex) true)
    (Variables|Default|SetcurrentGoal (+ (Variables|Default|GetcurrentGoal) 1))
    (if (< _returnvalue (Utilities|Array|Length _goals))
      (Rendering|SetActorHiddenInGame (Utilities|Array|Get(acopy) (Variables|Default|Getgoals) _returnvalue) false))))

(fn FinalGoallPassed
  (params (timestamp :type Float%20%28double-precision%29))
  (if (== (Variables|Default|GetcurrentGoal) (- (Utilities|Array|Length (Variables|Default|Getgoals)) 1))
    (Rendering|SetActorHiddenInGame true)
    (Default|ChooseTrophy (Variables|Default|GettrophyManager) (- timestamp (Variables|Default|GetbeginTimestamp)))))

(fn Reset
  (params (firstTime :type Boolean))
  (Variables|Default|SetcurrentGoal 0)
  (Variables|Default|SetbeginTimestamp (Utilities|Time|GetTimeSeconds))
  (for (_array_element _array_index) (Variables|Default|Getgoals)
    (if firstTime
      (Default|Init _array_element self _array_index))
    (Rendering|SetActorHiddenInGame _array_element true))
  (bind _index (Utilities|ForLoopLessThan 0 (Variables|Default|GetnumActive))
    (:LoopBody
      (Rendering|SetActorHiddenInGame (Utilities|Array|Get(acopy) (Variables|Default|Getgoals) _index) false))))