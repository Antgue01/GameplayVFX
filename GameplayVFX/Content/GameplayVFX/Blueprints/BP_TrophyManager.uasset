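; Trophy manager actor that picks and spawns a trophy based on the player's time.
; ChooseTrophy walks the keys of the TimesAndFx map for the first threshold the time fits, falling back to the last entry as the worst trophy.
; SpawnTrophy spawns a BP_Hat at the SpawnPos actor's transform and calls Init on it.
; BeginPlay only debug-prints data table column values, with no link to trophy selection.
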(event EventBeginPlay
  (bind _outrownames (DataTable|GetDataTableRowNames 0))
  (for _array_element _outrownames
    (bind _returnvalue (Class|DataTableFunctionLibrary|GetDataTableColumnasString 0 _array_element))
    (for _array_element_2 _returnvalue
      (Development|PrintString "Hello" true true "(R=0.002850,G=0.000000,B=1.000000,A=1.000000)" 1e+01)
      (Development|PrintString (Utilities|String|Append _array_element_2 "dsf")))))

(event Collision|EventActorBeginOverlap
  (params (OtherActor :type Actor%20Object%20Reference)))

(event EventTick
  (params (DeltaSeconds :type Float%20%28single-precision%29)))

(fn ConstructionScript)

(fn ChooseTrophy
  (params (playerTime :type Float%20%28double-precision%29))
  (bind _timesandfx (Variables|Default|GettimesAndFx))
  ;[0.02701 0.1684 0.04174] We find the right trophy based on the player time
  (while (and (< (LocalVariables|Geti) (Utilities|Map|Length _timesandfx)) (not (LocalVariables|Getspawned)))
    (bind _keys (Utilities|Map|Keys _timesandfx))
    (if (<= playerTime (Utilities|Array|Get(acopy) _keys (LocalVariables|Geti)))
      (LocalVariables|Setspawned true)
      (CallFunction|SpawnTrophy (.Value (Utilities|Map|Find (Variables|Default|GettimesAndFx) (Utilities|Array|Get(acopy) _keys (LocalVariables|Geti)))))
      (else
        (LocalVariables|Seti (+ (LocalVariables|Geti) 1)))))
  ;[0.02701 0.1684 0.04174] If the time is greater than all the values, we spawn the worst trophy
  (if (not (LocalVariables|Getspawned))
    (CallFunction|SpawnTrophy (.Value (Utilities|Map|Find (Variables|Default|GettimesAndFx) (Utilities|Array|Get(acopy) _keys (- (Utilities|Array|Length _keys) 1)))))))

(fn SpawnTrophy
  (params (trophy :type Niagara%20System%20Object%20Reference%20%28by%20ref%29))
  (bind _returnvalue (Game|SpawnActorfromClass "/Game/GameplayVFX/Blueprints/BP_Hat.BP_Hat_C" (Transformation|GetActorTransform (Variables|Default|GetSpawnPos)) "Undefined" 0 0))
  (bind _output_get (Variables|Default|Settrophy _returnvalue))
  (Default|Init _output_get trophy))