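; BP_TimeFeedback shifts a shared color over elapsed time, following time thresholds taken from the TrophyManager.
; BeginPlay builds the thresholds from zero plus each TimesAndFx key, offset by Tolerance.
; Tick blends neighboring Colors entries in HSV and writes the result to the "Color" parameter of a Material Parameter Collection.
; The mapped alpha slightly overshoots one to advance to the next color pair, stopping at the last color.
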(event EventBeginPlay
  (bind _times (Variables|Default|GetTimes))
  (CallFunction|Reset)
  (Utilities|Array|Add _times 0.0)
  (bind _keys (Utilities|Map|Keys (Variables|/Game/GameplayVFX/Blueprints/BP_TrophyManager.BP_TrophyManager_C|GettimesAndFx (Variables|Default|GetTrophyManager))))
  (for _array_element _keys
    (Utilities|Array|Add _times (+ _array_element (Variables|Default|GetTolerance)))))

(event Collision|EventActorBeginOverlap
  (params (OtherActor :type Actor%20Object%20Reference)))

(event EventTick
  (params (DeltaSeconds :type Float%20%28single-precision%29))
  (bind _times (Variables|Default|GetTimes))
  (bind _colors (Variables|Default|GetColors))
  (bind _output_get (Variables|Default|SetTime (+ (Variables|Default|GetTime) DeltaSeconds)))
  (Rendering|Material|SetVectorParameterValue (Variables|Default|GetParameterCollection) (Utilities|String|StringToName (Utilities|String|MakeLiteralString "Color")) (Class|KismetMathLibrary|LinearColorLerpUsingHSV (Utilities|Array|Get(acopy) _colors (Variables|Default|GetFirstIndex)) (Utilities|Array|Get(acopy) _colors (Variables|Default|GetSecondIndex)) (Math|Float|MapRangeClamped _output_get (Utilities|Array|Get(acopy) _times (Variables|Default|GetFirstIndex)) (Utilities|Array|Get(acopy) _times (Variables|Default|GetSecondIndex)) 0.0 1.01)) :!class /Script/Engine.KismetMaterialLibrary)
  (if (and (>= (Math|Float|MapRangeClamped _output_get (Utilities|Array|Get(acopy) _times (Variables|Default|GetFirstIndex)) (Utilities|Array|Get(acopy) _times (Variables|Default|GetSecondIndex)) 0.0 1.01) 1.0) (< (Variables|Default|GetSecondIndex) (- (Utilities|Array|Length _colors) 1)))
    (bind _output_get_2 (Variables|Default|SetFirstIndex (+ (Variables|Default|GetFirstIndex) 1)))
    (Variables|Default|SetSecondIndex (+ _output_get_2 1))))

(fn ConstructionScript)

(fn Reset
  (Variables|Default|SetFirstIndex 0)
  (Variables|Default|SetSecondIndex 1)
  (Variables|Default|SetTime 0.0))