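; BP_Hat is a hat pickup actor that any actor with a HatManager component can wear by touching it.
; On collider overlap, Wear destroys that actor's current hat, registers itself in the HatManager, flags itself as worn and snaps to the skeletal mesh's "hat" socket, keeping relative scale.
; A separate Init function spawns a supplied effect system attached to the hat's root and stores the spawned instance.
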(event OnComponentBeginOverlap(Collider)
  (params (OverlappedComponent :type Primitive%20Component%20Object%20Reference) (OtherActor :type Actor%20Object%20Reference) (OtherComp :type Primitive%20Component%20Object%20Reference) (OtherBodyIndex :type Integer) (bFromSweep :type Boolean) (SweepResult :type Hit%20Result%20Structure%20%28by%20ref%29))
  (CallFunction|Wear OtherActor))

(event EventBeginPlay)

(event Collision|EventActorBeginOverlap
  (params (OtherActor :type Actor%20Object%20Reference)))

(event EventTick
  (params (DeltaSeconds :type Float%20%28single-precision%29)))

(fn ConstructionScript)

(fn Init
  (params (Fx :type Niagara%20System%20Object%20Reference))
  (bind _returnvalue (Niagara|SpawnSystemAttached Fx (Variables|Default|GetDefaultSceneRoot) "None" (Transformation|GetActorLocation) "0, 0, 0" "KeepWorldPosition" false))
  (Variables|Default|Setfx _returnvalue))

(fn Wear
  (params (other :type Actor%20Object%20Reference))
  (bind _returnvalue (Actor|GetComponentbyClass other "/Game/GameplayVFX/Blueprints/HatManager.HatManager_C"))
  (if (Utilities|IsValid _returnvalue)
    (if (Utilities|IsValid (Variables|/Game/GameplayVFX/Blueprints/HatManager.HatManager_C|Gethat _returnvalue))
      (Actor|DestroyActor (Variables|/Game/GameplayVFX/Blueprints/HatManager.HatManager_C|Gethat _returnvalue)))
    (Variables|Default|SetbeingWorn true)
    (Variables|/Game/GameplayVFX/Blueprints/HatManager.HatManager_C|Sethat _returnvalue self)
    (Transformation|AttachComponentToComponent (Actor|GetComponentbyClass other "/Script/Engine.SkeletalMeshComponent") "hat" "SnapToTarget" "SnapToTarget" "KeepRelative" true)))